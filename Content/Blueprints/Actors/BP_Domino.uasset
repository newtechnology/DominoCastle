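; BP_Domino is a physics-simulated domino actor with velocity-driven impact and movement sounds, which can be reset to its starting transform.
; Construction applies the Static setting to physics and tick and picks a random domino or card material by type.
; Tick infers impacts from speed drops to play hit sounds, and runs a randomly offset movement sound with speed-scaled volume.
; Physics stops when a moving domino falls below a height limit.
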(event EventOnReset
  (bind _staticmesh (Variables|Default|GetStaticMesh))
  (Physics|SetSimulatePhysics _staticmesh false)
  (Transformation|SetActorTransform (Variables|Default|GetOriginalTransform) false true)
  (Physics|SetSimulatePhysics _staticmesh true)
  ;[1 1 1] Reset Simulation State
  (Variables|Default|SetOldUp false)
  (Variables|Default|SetOldVelocitylength 0.0)
  (Variables|Default|SetReadyForSoundSimulation false)
  (Variables|Default|SetInScene true)
  (CallFunction|SetStatic)
  (Audio|Components|Audio|Stop (Variables|Default|GetMovingDomino)))

(event EventTick
  (params (DeltaSeconds :type Float%20%28single-precision%29))
  (bind _returnvalue (Transformation|GetVelocity))
  (bind _maxfallspeed (Variables|Default|GetMaxFallSpeed))
  (bind _movingdomino (Variables|Default|GetMovingDomino))
  (bind _returnvalue_2 (Math|Vector|VectorLengthSquared _returnvalue))
  (bind _returnvalue_3 (Math|Float|Sqrt _returnvalue_2))
  (bind _returnvalue_4 (/ _returnvalue_3 _maxfallspeed))
  ;[1 1 1] Simmulation Starter/Stopper Qualifier
  (if (and (Variables|Default|GetInScene) (or (Variables|Default|GetReadyForSoundSimulation) (> _returnvalue_2 (Variables|Default|GetSquaredSimulationStarterVelocity))))
    (Variables|Default|SetReadyForSoundSimulation (> _returnvalue_2 (Variables|Default|GetSquaredSimulationStopperVelocity)))
    ;[1 1 1] Collision Check
    (if (Math|Boolean|ANDBoolean (Variables|Default|GetOldUp) (< _returnvalue_3 (Variables|Default|GetOldVelocitylength)) (< (- _returnvalue_3 (Variables|Default|GetOldVelocitylength)) (Variables|Default|GetMinImpactVelocity)))
      ;[1 1 1] On Collision
      (Audio|PlaySoundatLocation "/Game/SoundEffects/DominoHittingDomino.DominoHittingDomino" (Transformation|GetActorLocation) "0, 0, 0" _returnvalue_4 1.0 0.0 "/Game/SoundEffects/SoundAttenuation.SoundAttenuation")
      (Variables|Default|SetReadyForSoundSimulation false))
    ;[1 1 1] Old State Set
    (Variables|Default|SetOldVelocitylength _returnvalue_3)
    (Variables|Default|SetOldUp (not (< _returnvalue_3 (Variables|Default|GetOldVelocitylength))))
    ;[1 1 1] Play Move Sound
    (if (< (Variables|Default|GetMinMoveVelocity) _returnvalue_3)
      (if (not (Audio|Components|Audio|IsPlaying _movingdomino))
        (Audio|Components|Audio|SetVolumeMultiplier _movingdomino _returnvalue_4 :!class /Script/Engine.AudioComponent)
        (Audio|Components|Audio|Play _movingdomino (Math|Random|RandomFloatinRange 0.0 (Variables|Default|GetStartRandomizerConstant)))
        (elif (< (.Z (Math|Vector|BreakVector (Transformation|GetActorLocation))) (Variables|Default|GetMinZ))
          (Physics|SetSimulatePhysics (Variables|Default|GetStaticMesh) false)
          (Variables|Default|SetInScene false)))
      (else
        (Audio|Components|Audio|Stop _movingdomino)))))

(event EventBeginPlay
  (Variables|Default|SetOriginalTransform (Transformation|GetActorTransform)))

(fn ConstructionScript
  (bind _cardvariations (Variables|Default|GetCardVariations))
  (bind _dominovariations (Variables|Default|GetDominoVariations))
  (CallFunction|SetStatic)
  (switch int (Variables|Default|GetDominoType)
    (:0
      (bind _output_get (Variables|Default|SetDominoVariation (Math|Random|RandomIntegerinRange 0 (- (Utilities|Array|Length _dominovariations) 1))))
      (Rendering|Material|SetMaterial (Variables|Default|GetStaticMesh) 0 (Utilities|Array|Get(acopy) _dominovariations _output_get)))
    (:1
      (bind _output_get_2 (Variables|Default|SetDominoVariation (Math|Random|RandomIntegerinRange 0 (- (Utilities|Array|Length _cardvariations) 1))))
      (Rendering|Material|SetMaterial (Variables|Default|GetStaticMesh) 0 (Utilities|Array|Get(acopy) _cardvariations _output_get_2)))))

(fn SetStatic
  (bind _static (Variables|Default|GetStatic))
  (bind _returnvalue (not _static))
  (Physics|SetSimulatePhysics (Variables|Default|GetStaticMesh) _returnvalue)
  (Actor|Tick|SetActorTickEnabled _returnvalue))

(fn UnSetStatic
  (Physics|SetSimulatePhysics (Variables|Default|GetStaticMesh) true)
  (Actor|Tick|SetActorTickEnabled true))